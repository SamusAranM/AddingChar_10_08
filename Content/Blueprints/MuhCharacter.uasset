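; Player character that creates the HUD and handles movement, look, pause, projectile fire and a scattered flak alt-fire.
; Jumps spend Energy, which a Timeline refills after a short retriggerable delay.
; Store line-traces for "Source"-tagged components and records their actors in Pocket without removing them from the world.
; Unpack box-traces with the first entry's bounds, spawns a new actor of its class at the hit or maximum range, then drops the entry.
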(event `self.ReceiveBeginPlay`
  (bind _returnvalue (`|CreateWidget` "/Game/UI/MuhHUD.MuhHUD_C"))
  (bind _output_get (set `self.MuhHUD` _returnvalue))
  (`UserWidget.AddToViewport` _output_get 0)
  (`WidgetBlueprintLibrary.SetInputMode_GameOnly` (`GameplayStatics.GetPlayerController` 0)))

(event `InputAction|Fire`
  (params (Key :type "Key Structure"))
  (bind _returnvalue_location (`KismetMathLibrary.BreakTransform` (`self.GetTransform`)))
  ;[1 1 1] Fire?
  (:`Pressed`
    (`|SpawnActorFromClass` "/Game/Blueprints/MuhProjectile.MuhProjectile_C" (`KismetMathLibrary.MakeTransform` (+ (+ _returnvalue_location (0.0 0.0 50.0)) (* (`self.GetActorRightVector`) -75.0)) (`self.GetControlRotation`)) "Undefined" "OverrideRootScale" null null)))

(event `InputAction|Jump`
  (params (Key :type "Key Structure"))
  (bind _energy (`self.Energy`))
  ;[1 1 1] Character Movement
  (:`Pressed`
    (if (>= _energy 0.25)
      (set `self.Energy` (- _energy 0.25))
      (`self.Jump`)
      (`|ExecutionSequence`
        (:`then_0`
          (bind (_direction _cooldown) (`Timeline|Timeline_0` :!via `Stop` :!label _label)
            (:`Update`
              (set `self.Energy` (`KismetMathLibrary.Lerp` (`self.Energy`) 1.0 _cooldown)))))
        (:`then_1`
          (`KismetSystemLibrary.RetriggerableDelay` 0.2)
          (goto _label :!via `PlayFromStart`))))))

(event `InputAxis|Strafe`
  (params (AxisValue :type "Float (single-precision)"))
  ;[1 1 1] Character Movement
  (`self.AddMovementInput` (`self.GetActorRightVector`) AxisValue))

(event `InputAction|Pause`
  (params (Key :type "Key Structure"))
  ;[1 1 1] Character Movement
  (:`Pressed`
    (`/Engine/EditorBlueprintResources/StandardMacros.FlipFlop`
      (:`A`
        (`GameplayStatics.SetGamePaused` true))
      (:`B`
        (`GameplayStatics.SetGamePaused` false)))))

(event `InputAxis|Walk`
  (params (AxisValue :type "Float (single-precision)"))
  ;[1 1 1] Character Movement
  (`self.AddMovementInput` (`self.GetActorForwardVector`) AxisValue))

(event `InputAction|AltFire`
  (params (Key :type "Key Structure"))
  (bind _returnvalue_location (`KismetMathLibrary.BreakTransform` (`self.GetTransform`)))
  ;[1 1 1] Fire?
  (:`Pressed`
    (`MuhBPLibrary.FlakShot` "/Game/Blueprints/MuhProjectile.MuhProjectile_C" (+ (+ _returnvalue_location (0.0 0.0 50.0)) (* (`self.GetActorRightVector`) -75.0)) (`self.GetControlRotation`) 5 5 5.0 5.0)))

(event `InputAxis|LookV`
  (params (AxisValue :type "Float (single-precision)"))
  ;[1 1 1] Character Movement
  (`self.AddControllerPitchInput` AxisValue))

(event `InputAxis|LookH`
  (params (AxisValue :type "Float (single-precision)"))
  ;[1 1 1] Character Movement
  (`self.AddControllerYawInput` AxisValue))

(event `InputAction|Store`
  (params (Key :type "Key Structure"))
  (bind _returnvalue (`self.K2_GetActorLocation`))
  (bind _pocket (`self.Pocket`))
  ;[1 1 1] Spaghetti
  (:`Pressed`
    (bind _outhit (`KismetSystemLibrary.LineTraceSingleForObjects` :`Start` _returnvalue :`End` (+ _returnvalue (* (`KismetMathLibrary.Conv_RotatorToVector` (`self.GetControlRotation`)) 400.0)) :`ObjectTypes` (`self.TargetTypes`) :`DrawDebugType` "ForDuration" :`TraceColor` (struct :`R` 0.010252 :`G` 0.015914 :`B` 1.0 :`A` 1.0)))
    (if (`GameplayStatics.BreakHitResult` _outhit)
      (if (`ActorComponent.ComponentHasTag` (`.HitComponent` (`GameplayStatics.BreakHitResult` _outhit)) "Source")
        (if (not (`KismetArrayLibrary.Array_Contains` _pocket (`.HitActor` (`GameplayStatics.BreakHitResult` _outhit))))
          (`KismetArrayLibrary.Array_Insert` _pocket (`.HitActor` (`GameplayStatics.BreakHitResult` _outhit))))))))

(event `InputAction|Unpack`
  (params (Key :type "Key Structure"))
  (bind _returnvalue (`self.K2_GetActorLocation`))
  (bind _pocket (`self.Pocket`))
  (bind _output (`|GetArrayItem` (`self.Pocket`)))
  (bind _output_2 (`|GetArrayItem` _pocket))
  (bind _returnvalue_2 (+ _returnvalue (* (`KismetMathLibrary.Conv_RotatorToVector` (`self.GetControlRotation`)) 400.0)))
  ;[1 1 1] Spaghetti
  (:`Pressed`
    (if (`KismetSystemLibrary.IsValid` _output)
      (bind _outhit (`KismetSystemLibrary.BoxTraceSingle` :`Start` _returnvalue :`End` _returnvalue_2 :`HalfSize` (`.BoxExtent` (`self.GetActorBounds` _output false)) :`TraceChannel` "TraceTypeQuery2" :`DrawDebugType` "ForDuration"))
      (if (`GameplayStatics.BreakHitResult` _outhit)
        (if (`KismetSystemLibrary.IsValid` _output_2)
          (set `self.SpawnTarget` (`.Location` (`GameplayStatics.BreakHitResult` _outhit)))
          (`|SpawnActorFromClass` (`GameplayStatics.GetObjectClass` _output_2) (`KismetMathLibrary.MakeTransform` (`self.SpawnTarget`)) "Undefined" "OverrideRootScale" null null :!label _label_2)
          (`KismetArrayLibrary.Array_Remove` _pocket))
        (else
          (set `self.SpawnTarget` _returnvalue_2)
          (goto _label_2))))))

(fn `UserConstructionScript`)